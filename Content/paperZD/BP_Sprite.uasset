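; BP_Sprite is an actor in the paperZD folder that trails the player character when its IsFollowing flag is set.
; Each tick, if it is more than 200 units from player 0, it eases toward the player's location with a slow VInterpTo and SetActorLocation without sweep.
; Nothing in this Blueprint sets the flag, and BeginPlay and overlap events are unused.
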(event EventBeginPlay)

(event Collision|EventActorBeginOverlap
  (params (OtherActor :type Actor%20Object%20Reference)))

(event EventTick
  (params (DeltaSeconds :type Float%20%28single-precision%29))
  (bind _returnvalue (Transformation|GetActorLocation))
  (bind _returnvalue_2 (Game|GetPlayerCharacter 0))
  (bind _returnvalue_3 (Transformation|GetActorLocation _returnvalue_2))
  (if (Variables|Default|GetIsFollowing)
    (if (> (Math|Vector|Distance(Vector) _returnvalue _returnvalue_3) 2e+02)
      (Transformation|SetActorLocation (Math|Interpolation|VInterpTo _returnvalue _returnvalue_3 (Utilities|Time|GetWorldDeltaSeconds) 0.6) false false))))

(fn ConstructionScript)
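; BP_Char1 is a player-controlled character Blueprint that handles movement and a timed fight action through Enhanced Input.
; IA_Move feeds its two axes into movement along world X and Y and stores the input as MoveDirection.
; IA_Fight raises IsFighting and clears it after a fixed delay; nothing in this Blueprint reads either variable.
; Debug prints for X and Y values are left unconnected.
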(event Input|EnhancedActionEvents|EnhancedInputActionIA_Fight
  (params (ActionValue :type Boolean) (ElapsedSeconds :type Float%20%28double-precision%29) (TriggeredSeconds :type Float%20%28double-precision%29) (InputAction :type Input%20Action%20Object%20Reference :default "/Game/inputs/IA_Fight.IA_Fight"))
  (:Started
    (Variables|Default|SetIsFighting? true)
    (Utilities|FlowControl|Delay 2.4)
    (Variables|Default|SetIsFighting? false)))

(event Input|EnhancedActionEvents|EnhancedInputActionIA_Move
  (params (ActionValue :type Vector%202D%20Structure) (ElapsedSeconds :type Float%20%28double-precision%29) (TriggeredSeconds :type Float%20%28double-precision%29) (InputAction :type Input%20Action%20Object%20Reference :default "/Game/inputs/IA_Move.IA_Move"))
  (bind (_x _y) (Math|Vector2D|BreakVector2D ActionValue))
  (Pawn|Input|AddMovementInput "1.000000,0.000000,0.000000" _x false)
  (Pawn|Input|AddMovementInput "0.000000,1.000000,0.000000" _y false)
  (Variables|Default|SetMoveDirection ActionValue))

(event EventBeginPlay)

(event Collision|EventActorBeginOverlap
  (params (OtherActor :type Actor%20Object%20Reference)))

(event EventTick
  (params (DeltaSeconds :type Float%20%28single-precision%29)))

(fn ConstructionScript)
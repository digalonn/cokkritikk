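; BP_Dolap1 is an interactable 2D cabinet (dolap) that the player opens and closes with the E key.
; A Box overlap with BP_Char enables input on the actor and the end of the overlap disables it, so E only works nearby.
; Each press runs a FlipFlop that swaps the PaperSprite between the cabinet interior and cabinet door sprites.
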(event OnComponentBeginOverlap(Box)
  (params (OverlappedComponent :type Primitive%20Component%20Object%20Reference) (OtherActor :type Actor%20Object%20Reference) (OtherComp :type Primitive%20Component%20Object%20Reference) (OtherBodyIndex :type Integer) (bFromSweep :type Boolean) (SweepResult :type Hit%20Result%20Structure%20%28by%20ref%29))
  (Utilities|Casting|CastToBP_Char OtherActor)
  (Input|EnableInput (Game|GetPlayerController 0)))

(event OnComponentEndOverlap(Box)
  (params (OverlappedComponent :type Primitive%20Component%20Object%20Reference) (OtherActor :type Actor%20Object%20Reference) (OtherComp :type Primitive%20Component%20Object%20Reference) (OtherBodyIndex :type Integer))
  (Utilities|Casting|CastToBP_Char OtherActor)
  (Input|DisableInput (Game|GetPlayerController 0)))

(event EventBeginPlay)

(event Collision|EventActorBeginOverlap
  (params (OtherActor :type Actor%20Object%20Reference)))

(event EventTick
  (params (DeltaSeconds :type Float%20%28single-precision%29)))

(event Input|KeyboardEvents|E
  (params (Key :type Key%20Structure :default "None"))
  (bind _papersprite (Variables|Default|GetPaperSprite))
  (:Pressed
    (Utilities|FlowControl|FlipFlop
      (:A
        (Rendering|Components|Sprite|SetSprite _papersprite "/Game/Assets/saum_dolap_iç_Sprite.saum_dolap_iç_Sprite"))
      (:B
        (Rendering|Components|Sprite|SetSprite _papersprite "/Game/Assets/dolap_kapağı_Sprite_1.dolap_kapağı_Sprite_1")))))

(fn ConstructionScript)